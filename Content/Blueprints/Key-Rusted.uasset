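; Pickup actor for a rusted key that the player collects.
; Its PickUp event sets the KeyRusted flag on Agamenon, plays a key sound and destroys the actor.
; It then shows a found message through Agamenon's HUDLog and clears it after a short delay, with both steps placed after the DestroyActor call.
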(event `self.PickUp`
  (set `/Game/Blueprints/ThirdPersonCharacter.Key_Rusted` true (`self.Agamenon`))
  (`GameplayStatics.PlaySound2D` "/Game/Audio/Source/Keys.Keys" 1.0 1.0 0.0 null null)
  (`self.K2_DestroyActor`)
  (`/Game/Blueprints/ThirdPersonCharacter.HUDLog` (`self.Agamenon`) "Rusted Key found!")
  (`KismetSystemLibrary.Delay` 2.0)
  (`/Game/Blueprints/ThirdPersonCharacter.HUDLog` (`self.Agamenon`) ""))

(fn `UserConstructionScript`
  (`parent.UserConstructionScript`))