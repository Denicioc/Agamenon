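; Grandfather clock Blueprint that swings a static mesh component, likely its pendulum, back and forth from BeginPlay onward.
; An endless Delay-timed loop steps a counter between zero and an upper limit, adding a small pitch rotation on each step.
; A boolean flag flips at each limit to reverse direction, so the motion is linear and fixed-step rather than driven by Tick or a Timeline.
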(event `self.ReceiveBeginPlay`
  (bind _input (`self.Input`))
  (if (`self.Condition`) :!label _label
    (`/Engine/EditorBlueprintResources/StandardMacros.CompareInt` _input
      (:`>`
        (`/Engine/EditorBlueprintResources/StandardMacros.DecrementInt` _input
          (:`  `
            (`SceneComponent.K2_AddLocalRotation` (`self.StaticMesh1`) (`KismetMathLibrary.MakeRotator` 0.0 -0.2) false false)
            (`KismetSystemLibrary.Delay` 0.01)
            (goto _label))))
      (:`==`
        _)
      (:`<`
        _))
    (set `self.Condition` false)
    (goto _label)
    (else
      (`/Engine/EditorBlueprintResources/StandardMacros.CompareInt` _input 70
        (:`>`
          _)
        (:`==`
          _)
        (:`<`
          (`/Engine/EditorBlueprintResources/StandardMacros.IncrementInt` _input
            (:`  `
              (`SceneComponent.K2_AddLocalRotation` (`self.StaticMesh1`) (`KismetMathLibrary.MakeRotator` 0.0 0.2) false false)
              (`KismetSystemLibrary.Delay` 0.01)
              (goto _label)))))
      (set `self.Condition` true)
      (goto _label))))

(fn `UserConstructionScript`)