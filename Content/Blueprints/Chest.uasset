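; Interactable chest that opens and closes on the Interact input when the player has the rusted key, and otherwise shows a locked message on the HUD.
; Box overlap enables input and a gate, and each accepted press alternates open and close through a FlipFlop.
; Opening plays a door sound and grants coins only the first time.
; Delay-driven counter loops rotate the lid incrementally, with AnimCheck blocking presses mid-animation.
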(event `self.Box.OnComponentBeginOverlap`
  (params (OverlappedComponent :type "PrimitiveComponent Object Reference") (OtherActor :type "Actor Object Reference") (OtherComp :type "PrimitiveComponent Object Reference") (OtherBodyIndex :type Integer) (bFromSweep :type Boolean) (SweepResult :type "HitResult Structure (by ref)"))
  (bind _i (`self.I`))
  (bind _lid (`self.Lid`))
  (`self.EnableInput` (`GameplayStatics.GetPlayerController` 0))
  (goto _label :!via `Open`))

(event `InputAction|Interact`
  (params (Key :type "Key Structure"))
  (bind _i (`self.I`))
  (bind _lid (`self.Lid`))
  (:`Pressed`
    (`/Engine/EditorBlueprintResources/StandardMacros.Gate` true :!label _label
      (:`Exit`
        (if (not (`self.Anim Check`))
          (bind _output_get (set `self.Agamenon` (cast `/Game/Blueprints/ThirdPersonCharacter` (`GameplayStatics.GetPlayerCharacter` 0) :!pure true)))
          (if (`/Game/Blueprints/ThirdPersonCharacter.Key_Rusted` _output_get)
            (`/Engine/EditorBlueprintResources/StandardMacros.FlipFlop`
              (:`A`
                (`|ExecutionSequence`
                  (:`then_0`
                    (`GameplayStatics.PlaySound2D` "/Game/Audio/Source/wood-door.wood-door" 1.0 1.0 0.0 null null)
                    (`/Engine/EditorBlueprintResources/StandardMacros.DoOnce` false
                      (:`Completed`
                        (`/Game/Blueprints/ThirdPersonCharacter.ChangeCoin` (`self.Agamenon`) (`self.Amount`)))))
                  (:`then_1`
                    (`/Engine/EditorBlueprintResources/StandardMacros.CompareInt` _i 45 :!label _label_2
                      (:`>`
                        _)
                      (:`==`
                        _)
                      (:`<`
                        (`/Engine/EditorBlueprintResources/StandardMacros.IncrementInt` _i
                          (:`  `
                            (set `self.Anim Check` true)
                            (`SceneComponent.K2_AddLocalRotation` _lid (struct :`Pitch` 1.0) false false)
                            (`KismetSystemLibrary.Delay` 0.01)
                            (goto _label_2)))))
                    (set `self.Anim Check` false))))
              (:`B`
                (`/Engine/EditorBlueprintResources/StandardMacros.CompareInt` _i :!label _label_3
                  (:`>`
                    (`/Engine/EditorBlueprintResources/StandardMacros.DecrementInt` _i
                      (:`  `
                        (set `self.Anim Check` true)
                        (`SceneComponent.K2_AddLocalRotation` _lid (struct :`Pitch` -1.0) false false)
                        (`KismetSystemLibrary.Delay` 0.01)
                        (goto _label_3))))
                  (:`==`
                    _)
                  (:`<`
                    _))
                (set `self.Anim Check` false)))
            (else
              (`/Game/Blueprints/ThirdPersonCharacter.HUDLog` _output_get "This chest is locked! Rusted key required"))))))))

(event `self.Box.OnComponentEndOverlap`
  (params (OverlappedComponent :type "PrimitiveComponent Object Reference") (OtherActor :type "Actor Object Reference") (OtherComp :type "PrimitiveComponent Object Reference") (OtherBodyIndex :type Integer))
  (`self.DisableInput` (`GameplayStatics.GetPlayerController` 0))
  (goto _label :!via `Close`))

(fn `UserConstructionScript`)