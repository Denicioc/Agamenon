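; Door actor that the player opens and closes with the Interact input while inside a Box trigger.
; Overlapping the box enables input and opens a gate, and leaving disables input and closes it.
; A FlipFlop alternates opening and closing, rotating the mesh incrementally through delayed loops driven by a step counter.
; The AnimCheck flag blocks new presses while the door is moving.
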(event `self.Box.OnComponentBeginOverlap`
  (params (OverlappedComponent :type "PrimitiveComponent Object Reference") (OtherActor :type "Actor Object Reference") (OtherComp :type "PrimitiveComponent Object Reference") (OtherBodyIndex :type Integer) (bFromSweep :type Boolean) (SweepResult :type "HitResult Structure (by ref)"))
  (bind _i (`self.i`))
  (bind _staticmesh (`self.StaticMesh`))
  (`self.EnableInput` (`GameplayStatics.GetPlayerController` 0))
  (goto _label :!via `Open`))

(event `InputAction|Interact`
  (params (Key :type "Key Structure"))
  (bind _i (`self.i`))
  (bind _staticmesh (`self.StaticMesh`))
  (:`Pressed`
    (`/Engine/EditorBlueprintResources/StandardMacros.Gate` true :!label _label
      (:`Exit`
        (if (not (`self.Anim_check`))
          (`/Engine/EditorBlueprintResources/StandardMacros.FlipFlop`
            (:`A`
              (`/Engine/EditorBlueprintResources/StandardMacros.CompareInt` _i 30 :!label _label_2
                (:`>`
                  _)
                (:`==`
                  _)
                (:`<`
                  (`/Engine/EditorBlueprintResources/StandardMacros.IncrementInt` _i
                    (:`  `
                      (set `self.Anim_check` true)
                      (`SceneComponent.K2_AddLocalRotation` _staticmesh (struct :`Yaw` 3.0) false false)
                      (`KismetSystemLibrary.Delay` 0.001)
                      (goto _label_2)))))
              (set `self.Anim_check` false))
            (:`B`
              (`/Engine/EditorBlueprintResources/StandardMacros.CompareInt` _i :!label _label_3
                (:`>`
                  (`/Engine/EditorBlueprintResources/StandardMacros.DecrementInt` _i
                    (:`  `
                      (set `self.Anim_check` true)
                      (`SceneComponent.K2_AddLocalRotation` _staticmesh (struct :`Yaw` -3.0) false false)
                      (`KismetSystemLibrary.Delay` 0.001)
                      (goto _label_3))))
                (:`==`
                  _)
                (:`<`
                  _))
              (set `self.Anim_check` false))))))))

(event `self.Box.OnComponentEndOverlap`
  (params (OverlappedComponent :type "PrimitiveComponent Object Reference") (OtherActor :type "Actor Object Reference") (OtherComp :type "PrimitiveComponent Object Reference") (OtherBodyIndex :type Integer))
  (`self.DisableInput` (`GameplayStatics.GetPlayerController` 0))
  (goto _label :!via `Close`))

(fn `UserConstructionScript`)