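; Health flask pickup that restores the life of the Agamenon character.
; On PickUp it calls ChangeLife on Agamenon with LifeAmount, spawns the flask sound at world origin, destroys itself and logs a feel-better message to the HUD.
; It also defines its own ChangeLife, which adds directly to Agamenon's Life and returns it as text, plus a generic CustomInputSum increment helper, neither invoked by PickUp.
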(event `self.PickUp`
  (`/Game/Blueprints/ThirdPersonCharacter.ChangeLife` (`self.Agamenon`) (`self.LifeAmount`))
  (`GameplayStatics.SpawnSoundAtLocation` "/Game/Audio/Source/Flask.Flask" (0.0 0.0 0.0) (struct) 1.0 1.0 0.0 null null)
  (`self.K2_DestroyActor`)
  (`/Game/Blueprints/ThirdPersonCharacter.HUDLog` (`self.Agamenon`) "I feel much better!"))

(fn `ChangeLife`
  (params (PtVida :type Integer))
  (returns (ReturnValue :type Text))
  (bind _life (`/Game/Blueprints/ThirdPersonCharacter.Life` (`self.Agamenon`)))
  (`KismetSystemLibrary.PrintText` "I feel much better!")
  (bind _result (`/Engine/EditorBlueprintResources/StandardMacros.ManipulateIntInternal` _life (+ _life PtVida))
    (:`  `
      (return (`KismetTextLibrary.Conv_IntToText` _result)))))

(fn `UserConstructionScript`
  (`parent.UserConstructionScript`))