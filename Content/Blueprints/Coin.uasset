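; A collectible coin actor that spins and bobs in place until picked up.
; From BeginPlay, a self-repeating short Delay loop rotates the mesh and offsets its height from the starting position using a wrapping curve sample.
; PickUp speeds up the spin and curve playback, waits briefly, then uses DoOnce to play a sound, call ChangeCoin on Agamenon and destroy the actor.
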(event `self.ReceiveBeginPlay`
  (bind _staticmesh (`self.StaticMesh`))
  (bind _in_time (`self.In Time`))
  (bind (_initial_location_x _initial_location_y _initial_location_z) (`KismetMathLibrary.BreakVector` (`self.Initial Location`)))
  (set `self.Initial Location` (`SceneComponent.RelativeLocation` _staticmesh))
  (`SceneComponent.K2_SetRelativeLocation` _staticmesh (`KismetMathLibrary.MakeVector` _initial_location_x _initial_location_y (+ _initial_location_z (`CurveFloat.GetFloatValue` (`self.Curve`) _in_time))) false false :!label _label)
  (`SceneComponent.K2_AddLocalRotation` _staticmesh (`KismetMathLibrary.MakeRotator` (`self.Delta Rotation X (Roll)`)) false false)
  (bind _output_get (set `self.In Time` (+ _in_time (`self.Time`))))
  (if (> _output_get 2.0)
    (set `self.In Time` 0.0))
  (`KismetSystemLibrary.Delay` 0.02)
  (goto _label))

(event `self.PickUp`
  (set `self.Time` 0.2)
  (set `self.Delta Rotation X (Roll)` 25.0)
  (set `self.In Time` 2.0)
  (`KismetSystemLibrary.Delay` 0.2)
  (`/Engine/EditorBlueprintResources/StandardMacros.DoOnce` false
    (:`Completed`
      (`GameplayStatics.PlaySound2D` "/Game/Audio/Source/Coin2.Coin2" 1.0 1.0 0.0 null null false)
      (`/Game/Blueprints/ThirdPersonCharacter.ChangeCoin` (`self.Agamenon`) 1)
      (`self.K2_DestroyActor`))))

(fn `UserConstructionScript`
  (`parent.UserConstructionScript`))