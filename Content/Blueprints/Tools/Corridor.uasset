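; Corridor tool actor that procedurally builds a tiled tunnel section from Deep, Length and Height, with no runtime logic.
; The construction script creates separate dynamic instances of M_WormTunnels for floor, walls and ceiling.
; Nested loops then add static mesh components on a 100-unit grid, rotating tiles to form the floor, two side walls and ceiling, leaving the ends open.
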(fn `UserConstructionScript`
  (`|ExecutionSequence`
    (:`then_0`
      (bind _returnvalue (`KismetMaterialLibrary.CreateDynamicMaterialInstance` "/Game/Materials/M_WormTunnels.M_WormTunnels"))
      (set `self.MatFloor` _returnvalue)
      (bind _returnvalue_2 (`KismetMaterialLibrary.CreateDynamicMaterialInstance` "/Game/Materials/M_WormTunnels.M_WormTunnels"))
      (set `self.MatWall` _returnvalue_2)
      (bind _returnvalue_3 (`KismetMaterialLibrary.CreateDynamicMaterialInstance` "/Game/Materials/M_WormTunnels.M_WormTunnels"))
      (set `self.MatCeiling` _returnvalue_3))
    (:`then_1`
      ;[1 1 1] Floor
      (for _index (range (+ (`self.Deep`) 1))
        (bind _returnvalue_4 (* _index 100.0))
        (bind _returnvalue_5 (`AddComponent|NODE_AddStaticMeshComponent-0` :`RelativeTransform` (`KismetMathLibrary.MakeTransform` (`KismetMathLibrary.MakeVector` _returnvalue_4))))
        (`PrimitiveComponent.SetMaterial` _returnvalue_5 0 (`self.MatFloor`))
        (for _index_2 (range (+ (`self.Length`) 1))
          (bind _returnvalue_6 (`AddComponent|NODE_AddStaticMeshComponent-1` :`RelativeTransform` (`KismetMathLibrary.MakeTransform` (`KismetMathLibrary.MakeVector` _returnvalue_4 (* _index_2 100.0)))))
          (`PrimitiveComponent.SetMaterial` _returnvalue_6 0 (`self.MatFloor`))))
      ;[1 1 1] Wall Side 1
      (for _index_3 (range (+ (`self.Deep`) 1))
        (bind _returnvalue_7 (* _index_3 100.0))
        (bind _returnvalue_8 (`AddComponent|NODE_AddStaticMeshComponent-6` :`RelativeTransform` (`KismetMathLibrary.MakeTransform` (`KismetMathLibrary.MakeVector` _returnvalue_7 0.0 100.0) (struct :`Roll` 90.0))))
        (`PrimitiveComponent.SetMaterial` _returnvalue_8 0 (`self.MatWall`))
        (for _index_4 (range 1 (+ (`self.Height`) 1))
          (bind _returnvalue_9 (`AddComponent|NODE_AddStaticMeshComponent-7` :`RelativeTransform` (`KismetMathLibrary.MakeTransform` (`KismetMathLibrary.MakeVector` _returnvalue_7 0.0 (* _index_4 100.0)) (struct :`Roll` 90.0))))
          (`PrimitiveComponent.SetMaterial` _returnvalue_9 0 (`self.MatWall`))))
      ;[1 1 1] Wall Side 2
      (for _index_5 (range (+ (`self.Deep`) 1))
        (bind _returnvalue_10 (* (+ _index_5 -1) 100.0))
        (bind _returnvalue_11 (`AddComponent|NODE_AddStaticMeshComponent-8` :`RelativeTransform` (`KismetMathLibrary.MakeTransform` (`KismetMathLibrary.MakeVector` _returnvalue_10 (* (+ (`self.Length`) 1) 100.0) 100.0) (struct :`Yaw` 180.0 :`Roll` 90.0))))
        (`PrimitiveComponent.SetMaterial` _returnvalue_11 0 (`self.MatWall`))
        (for _index_6 (range 1 (+ (`self.Height`) 1))
          (bind _returnvalue_12 (`AddComponent|NODE_AddStaticMeshComponent-9` :`RelativeTransform` (`KismetMathLibrary.MakeTransform` (`KismetMathLibrary.MakeVector` _returnvalue_10 (* (+ (`self.Length`) 1) 100.0) (* _index_6 100.0)) (struct :`Yaw` 180.0 :`Roll` 90.0))))
          (`PrimitiveComponent.SetMaterial` _returnvalue_12 0 (`self.MatWall`))))
      ;[1 1 1] Ceiling
      (for _index_7 (range (+ (`self.Deep`) 1))
        (bind _returnvalue_13 (* (+ _index_7 -1) 100.0))
        (bind _returnvalue_14 (`AddComponent|NODE_AddStaticMeshComponent-4` :`RelativeTransform` (`KismetMathLibrary.MakeTransform` (`KismetMathLibrary.MakeVector` _returnvalue_13 0.0 (* (`self.Height`) 100.0)) (struct :`Pitch` 180.0))))
        (`PrimitiveComponent.SetMaterial` _returnvalue_14 0 (`self.MatCeiling`))
        (for _index_8 (range (+ (`self.Length`) 1))
          (bind _returnvalue_15 (`AddComponent|NODE_AddStaticMeshComponent-5` :`RelativeTransform` (`KismetMathLibrary.MakeTransform` (`KismetMathLibrary.MakeVector` _returnvalue_13 (* _index_8 100.0) (* (`self.Height`) 100.0)) (struct :`Pitch` 180.0))))
          (`PrimitiveComponent.SetMaterial` _returnvalue_15 0 (`self.MatCeiling`)))))))