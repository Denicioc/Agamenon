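; Spline-driven fence tool that builds a fence along its Spline component in the construction script.
; Static mesh posts are placed every Dist units along the spline length, using its world-space rotation plus a 90-degree local turn.
; Two further loops over the spline points add spline mesh rails at a lower and an upper height, bent with each point's local location and tangent.
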(fn `UserConstructionScript`
  (bind _spline (`self.Spline`))
  (bind _spline_2 (`self.Spline`))
  (bind _spline_3 (`self.Spline`))
  (for _index (range (+ (`KismetMathLibrary.FTrunc` (/ (`SplineComponent.GetSplineLength` _spline_2) (`self.Dist`))) 1))
    (bind _returnvalue (* _index (`self.Dist`)))
    (bind _returnvalue_2 (`AddComponent|NODE_AddStaticMeshComponent-0` :`RelativeTransform` (`KismetMathLibrary.MakeTransform` (`SplineComponent.GetLocationAtDistanceAlongSpline` _spline _returnvalue "Local") (`SplineComponent.GetRotationAtDistanceAlongSpline` _spline _returnvalue "World"))))
    (`SceneComponent.K2_AddLocalRotation` _returnvalue_2 (struct :`Yaw` 90.0) false false))
  (for _index_2 (range (+ (`SplineComponent.GetNumberOfSplinePoints` _spline_2) 1))
    (bind _returnvalue_3 (`AddComponent|NODE_AddSplineMeshComponent-0` :`RelativeTransform` (`KismetMathLibrary.MakeTransform` (0.0 0.0 50.0))))
    (bind (_location _tangent) (`SplineComponent.GetLocationAndTangentAtSplinePoint` _spline_2 _index_2 "Local"))
    (bind (_location_2 _tangent_2) (`SplineComponent.GetLocationAndTangentAtSplinePoint` _spline_2 (+ _index_2 1) "Local"))
    (`SplineMeshComponent.SetStartAndEnd` _returnvalue_3 _location _tangent _location_2 _tangent_2 true))
  (for _index_3 (range (+ (`SplineComponent.GetNumberOfSplinePoints` _spline_3) 1))
    (bind _returnvalue_4 (`AddComponent|NODE_AddSplineMeshComponent-1` :`RelativeTransform` (`KismetMathLibrary.MakeTransform` (0.0 0.0 250.0))))
    (bind (_location_3 _tangent_3) (`SplineComponent.GetLocationAndTangentAtSplinePoint` _spline_3 _index_3 "Local"))
    (bind (_location_4 _tangent_4) (`SplineComponent.GetLocationAndTangentAtSplinePoint` _spline_3 (+ _index_3 1) "Local"))
    (`SplineMeshComponent.SetStartAndEnd` _returnvalue_4 _location_3 _tangent_3 _location_4 _tangent_4 true)))