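; SP_Vine is a spline tool Blueprint that lays a mesh, presumably a vine, along an editable spline.
; The construction script splits the spline length into segments of Dist and adds a spline mesh component for each, using the configured Mesh and Material.
; Each segment takes its endpoints and tangents from the spline, with tangent length clamped to Dist, and applies a uniform cross-section Scale.
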(fn `UserConstructionScript`
  (locals (NewLocalVar_0 :type "Float (double-precision)" :default 1.0))
  (bind _scale (`self.Scale`))
  (bind _scale_2 (`self.Scale`))
  (bind _spline (`self.Spline`))
  (bind _dist (`self.Dist`))
  (bind _spline_2 (`self.Spline`))
  (for _index (range (+ (`KismetMathLibrary.FTrunc` (/ (`SplineComponent.GetSplineLength` (`self.Spline`)) (`self.Dist`))) 1))
    (bind _returnvalue (`AddComponent|NODE_AddSplineMeshComponent-0`))
    (`StaticMeshComponent.SetStaticMesh` _returnvalue (`self.Mesh`))
    (`PrimitiveComponent.SetMaterial` _returnvalue 0 (`self.Material`))
    (bind _returnvalue_2 (* _index (`self.Dist`)))
    (bind _returnvalue_3 (* (+ _index 1) (`self.Dist`)))
    (`SplineMeshComponent.SetStartAndEnd` _returnvalue (`SplineComponent.GetLocationAtDistanceAlongSpline` _spline _returnvalue_2 "Local") (`KismetMathLibrary.ClampVectorSize` (`SplineComponent.GetTangentAtDistanceAlongSpline` _spline _returnvalue_2 "Local") 0.0 _dist) (`SplineComponent.GetLocationAtDistanceAlongSpline` _spline_2 _returnvalue_3 "Local") (`KismetMathLibrary.ClampVectorSize` (`SplineComponent.GetTangentAtDistanceAlongSpline` _spline_2 _returnvalue_3 "Local") 0.0 _dist) true)
    (`SplineMeshComponent.SetStartScale` _returnvalue (`KismetMathLibrary.MakeVector2D` _scale _scale) true)
    (`SplineMeshComponent.SetEndScale` _returnvalue (`KismetMathLibrary.MakeVector2D` _scale_2 _scale_2) true)))