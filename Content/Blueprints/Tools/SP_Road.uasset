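; SP_Road is a spline-driven road tool that builds a mesh road along an editable spline in the construction script.
; It creates a dynamic material instance with U, V and rotation parameters.
; It then places spline mesh components at fixed distance intervals, each using that material and a uniform cross-section scale.
; Tangents are clamped to the segment length so each piece bends cleanly along the curve.
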(fn `UserConstructionScript`
  (locals (NewLocalVar_0 :type "Float (double-precision)" :default 1.0))
  (bind _scale (`self.Scale`))
  (bind _scale_2 (`self.Scale`))
  (bind _spline (`self.Spline`))
  (bind _dist (`self.Dist`))
  (bind _spline_2 (`self.Spline`))
  (`|ExecutionSequence`
    (:`then_0`
      (bind _returnvalue (`KismetMaterialLibrary.CreateDynamicMaterialInstance` (`self.ParentInstance`)))
      (bind _output_get (set `self.Material` _returnvalue))
      (`MaterialInstanceDynamic.SetScalarParameterValue` _output_get "U" (`self.Mat_U`))
      (`MaterialInstanceDynamic.SetScalarParameterValue` _output_get "v" (`self.Mat_V`))
      (`MaterialInstanceDynamic.SetScalarParameterValue` _output_get "Rot" (`self.Mat_Rot`)))
    (:`then_1`
      (for _index (range (+ (`KismetMathLibrary.FTrunc` (/ (`SplineComponent.GetSplineLength` (`self.Spline`)) (`self.Dist`))) 1))
        (bind _returnvalue_2 (`AddComponent|NODE_AddSplineMeshComponent-0`))
        (`StaticMeshComponent.SetStaticMesh` _returnvalue_2 (`self.Mesh`))
        (`PrimitiveComponent.SetMaterial` _returnvalue_2 0 (`self.Material`))
        (bind _returnvalue_3 (* _index (`self.Dist`)))
        (bind _returnvalue_4 (* (+ _index 1) (`self.Dist`)))
        (`SplineMeshComponent.SetStartAndEnd` _returnvalue_2 (`SplineComponent.GetLocationAtDistanceAlongSpline` _spline _returnvalue_3 "Local") (`KismetMathLibrary.ClampVectorSize` (`SplineComponent.GetTangentAtDistanceAlongSpline` _spline _returnvalue_3 "Local") 0.0 _dist) (`SplineComponent.GetLocationAtDistanceAlongSpline` _spline_2 _returnvalue_4 "Local") (`KismetMathLibrary.ClampVectorSize` (`SplineComponent.GetTangentAtDistanceAlongSpline` _spline_2 _returnvalue_4 "Local") 0.0 _dist) true)
        (`SplineMeshComponent.SetStartScale` _returnvalue_2 (`KismetMathLibrary.MakeVector2D` _scale _scale) true)
        (`SplineMeshComponent.SetEndScale` _returnvalue_2 (`KismetMathLibrary.MakeVector2D` _scale_2 _scale_2) true)))))