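; Pebble is a tool Blueprint that varies the look of each placed pebble by randomizing a static mesh in the Construction Script.
; It picks a random mesh from an array and sets a random relative location, uniform plus per-axis scale, and rotation.
; Rotation comes from a random X-direction vector rather than Euler angles.
; The randomness is unseeded, so results re-roll whenever construction reruns; the event graph is empty.
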(fn `UserConstructionScript`
  (bind _meshes (`self.Meshes`))
  (bind (_rotx_x _rotx_y) (`KismetMathLibrary.BreakVector2D` (`self.RotX`)))
  (bind (_roty_x _roty_y) (`KismetMathLibrary.BreakVector2D` (`self.RotY`)))
  (bind (_rotz_x _rotz_y) (`KismetMathLibrary.BreakVector2D` (`self.RotZ`)))
  (bind (_uniformscale_x _uniformscale_y) (`KismetMathLibrary.BreakVector2D` (`self.UniformScale`)))
  (bind (_nonuniformscale_x _nonuniformscale_y _nonuniformscale_z) (`KismetMathLibrary.BreakVector` (`self.NonUniformScale`)))
  (bind (_locationrandom_x _locationrandom_y _locationrandom_z) (`KismetMathLibrary.BreakVector` (`self.LocationRandom`)))
  (`StaticMeshComponent.SetStaticMesh` (`self.StaticMesh`) (`|GetArrayItem` _meshes (`KismetMathLibrary.RandomIntegerInRange` 0 (`KismetArrayLibrary.Array_LastIndex` _meshes))))
  (`SceneComponent.K2_SetRelativeTransform` (`self.StaticMesh`) (`KismetMathLibrary.MakeTransform` (+ (* (1.0 1.0 1.0) 1.0) (`KismetMathLibrary.MakeVector` (`KismetMathLibrary.RandomFloatInRange` (* _locationrandom_x -1.0) _locationrandom_x) (`KismetMathLibrary.RandomFloatInRange` (* _locationrandom_y -1.0) _locationrandom_y) (`KismetMathLibrary.RandomFloatInRange` (* _locationrandom_z -1.0) _locationrandom_z))) (`KismetMathLibrary.Conv_VectorToRotator` (+ (* (1.0 1.0 1.0) 1.0) (`KismetMathLibrary.MakeVector` (`KismetMathLibrary.RandomFloatInRange` _rotx_x _rotx_y) (`KismetMathLibrary.RandomFloatInRange` _roty_x _roty_y) (`KismetMathLibrary.RandomFloatInRange` _rotz_x _rotz_y)))) (+ (* (1.0 1.0 1.0) (`KismetMathLibrary.RandomFloatInRange` _uniformscale_x _uniformscale_y)) (`KismetMathLibrary.MakeVector` (`KismetMathLibrary.RandomFloatInRange` (* _nonuniformscale_x -1.0) _nonuniformscale_x) (`KismetMathLibrary.RandomFloatInRange` (* _nonuniformscale_y -1.0) _nonuniformscale_y) (`KismetMathLibrary.RandomFloatInRange` (* _nonuniformscale_z -1.0) _nonuniformscale_z)))) false false))