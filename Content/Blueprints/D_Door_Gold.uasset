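; Gold-key double door that the player opens and closes with Interact while inside its trigger box.
; Overlap enables input and opens a gate; each press checks the character's KeyGold flag, logging a locked message if it is missing.
; A FlipFlop alternates directions, and a counter-driven Delay loop rotates both meshes oppositely in small steps, with a busy flag blocking presses mid-swing.
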(event `self.ReceiveBeginPlay`
  (set `self.Agamenon` (cast `/Game/Blueprints/ThirdPersonCharacter` (`GameplayStatics.GetPlayerCharacter` 0) :!pure true))
  (bind _returnvalue (`|CreateWidget` "/Game/UI/HUD/HUD.HUD_C"))
  (set `self.HUD` _returnvalue))

(event `self.Box.OnComponentBeginOverlap`
  (params (OverlappedComponent :type "PrimitiveComponent Object Reference") (OtherActor :type "Actor Object Reference") (OtherComp :type "PrimitiveComponent Object Reference") (OtherBodyIndex :type Integer) (bFromSweep :type Boolean) (SweepResult :type "HitResult Structure (by ref)"))
  (bind _agamenon (`self.Agamenon`))
  (bind _input (`self.Input`))
  (`self.EnableInput` (`GameplayStatics.GetPlayerController` 0))
  (goto _label :!via `Open`))

(event `InputAction|Interact`
  (params (Key :type "Key Structure"))
  (bind _agamenon (`self.Agamenon`))
  (bind _input (`self.Input`))
  (:`Pressed`
    (`/Engine/EditorBlueprintResources/StandardMacros.Gate` true :!label _label
      (:`Exit`
        (if (`self.Condition`)
          _
          (elif (`/Game/Blueprints/ThirdPersonCharacter.Key_gold` _agamenon)
            (`/Engine/EditorBlueprintResources/StandardMacros.FlipFlop`
              (:`A`
                (`/Engine/EditorBlueprintResources/StandardMacros.CompareInt` _input 30 :!label _label_2
                  (:`>`
                    _)
                  (:`==`
                    _)
                  (:`<`
                    (set `self.Condition` true)
                    (`/Engine/EditorBlueprintResources/StandardMacros.IncrementInt` _input
                      (:`  `
                        (`|ExecutionSequence`
                          (:`then_0`
                            (`SceneComponent.K2_AddLocalRotation` (`self.StaticMesh`) (struct :`Yaw` 3.0) false false))
                          (:`then_1`
                            (`SceneComponent.K2_AddLocalRotation` (`self.StaticMesh1`) (struct :`Yaw` -3.0) false false)))
                        (`KismetSystemLibrary.Delay` 0.01)
                        (goto _label_2)))))
                (set `self.Condition` false))
              (:`B`
                (`/Engine/EditorBlueprintResources/StandardMacros.CompareInt` _input :!label _label_3
                  (:`>`
                    (set `self.Condition` true)
                    (`/Engine/EditorBlueprintResources/StandardMacros.DecrementInt` _input
                      (:`  `
                        (`|ExecutionSequence`
                          (:`then_0`
                            (`SceneComponent.K2_AddLocalRotation` (`self.StaticMesh`) (struct :`Yaw` -3.0) false false))
                          (:`then_1`
                            (`SceneComponent.K2_AddLocalRotation` (`self.StaticMesh1`) (struct :`Yaw` 3.0) false false)))
                        (`KismetSystemLibrary.Delay` 0.01)
                        (goto _label_3))))
                  (:`==`
                    _)
                  (:`<`
                    _))
                (set `self.Condition` false)))
            (else
              (`/Game/Blueprints/ThirdPersonCharacter.HUDLog` _agamenon "The door is locked! Gold key required"))))))))

(event `self.Box.OnComponentEndOverlap`
  (params (OverlappedComponent :type "PrimitiveComponent Object Reference") (OtherActor :type "Actor Object Reference") (OtherComp :type "PrimitiveComponent Object Reference") (OtherBodyIndex :type Integer))
  (`self.DisableInput` (`GameplayStatics.GetPlayerController` 0))
  (goto _label :!via `Close`))

(fn `UserConstructionScript`
  (`parent.UserConstructionScript`))